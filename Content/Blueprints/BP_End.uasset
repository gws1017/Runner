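; BP_End is a level-end trigger that finishes the game once the player has collected the maximum fire.
; When the Main_BP player overlaps its Box with CurrentFire equal to MaxFire, it sets the player's MovementStatus to another state.
; It then removes all widgets, shows the HUDOverlayEnd screen and enables the mouse cursor.
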(event OnComponentBeginOverlap(Box)
  (params (OverlappedComponent :type Primitive%20Component%20Object%20Reference) (OtherActor :type Actor%20Object%20Reference) (OtherComp :type Primitive%20Component%20Object%20Reference) (OtherBodyIndex :type Integer) (bFromSweep :type Boolean) (SweepResult :type Hit%20Result%20Structure%20%28by%20ref%29))
  (bind _asmain_bp (Utilities|Casting|CastToMain_BP OtherActor))
  (if (== (Variables|/Game/Blueprints/Character/Main_BP.Main_BP_C|GetMaxFire _asmain_bp) (Variables|/Game/Blueprints/Character/Main_BP.Main_BP_C|GetCurrentFire _asmain_bp))
    (Variables|/Game/Blueprints/Character/Main_BP.Main_BP_C|SetMovementStatus _asmain_bp "NewEnumerator2")
    (Viewport|RemoveAllWidgets)
    (bind _returnvalue (UserInterface|CreateWidget "/Game/HUD/HUDOverlayEnd.HUDOverlayEnd_C"))
    (UserInterface|Viewport|AddtoViewport _returnvalue 0)
    (Variables|/Script/Engine.PlayerController|SetbShowMouseCursor (Game|GetPlayerController 0) true)))

(event EventBeginPlay)

(event Collision|EventActorBeginOverlap
  (params (OtherActor :type Actor%20Object%20Reference)))

(event EventTick
  (params (DeltaSeconds :type Float%20%28single-precision%29)))

(fn ConstructionScript)