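; BasicGameMode is a game mode that keeps a minutes-and-seconds timer and persists it to a save slot.
; BeginPlay caches the player pawn as Main_BP, and Tick uses a one-second Delay to advance the timer only while its MovementStatus equals the enum's NewEnumerator0.
; SaveData loads or creates a DataObject save and writes the time through its LoadTime function, while LoadData restores it; neither is called within this Blueprint.
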(event EventBeginPlay
  (bind _asmain_bp (Utilities|Casting|CastToMain_BP (Game|Player|GetPlayerPawn 0)))
  (Variables|Default|SetAs%20Main%20BP _asmain_bp))

(event EventTick
  (params (DeltaSeconds :type Float%20%28single-precision%29))
  (Utilities|FlowControl|Delay 1.0)
  (if (Utilities|Enum|Equal(Enum) (Variables|/Game/Blueprints/Character/Main_BP.Main_BP_C|GetMovementStatus (Variables|Default|GetAs%20Main%20BP)) "NewEnumerator0")
    (bind _result (Math|Integer|IncrementInt (Variables|Default|GetTimeSec))
      (:%20%20
        (Variables|Default|SetTimeSec _result)
        (if (> (Variables|Default|GetTimeSec) 59)
          (bind _result_2 (Math|Integer|IncrementInt (Variables|Default|GetTimeMin))
            (:%20%20
              (Variables|Default|SetTimeMin _result_2)
              (Variables|Default|SetTimeSec 0))))))))

(fn ConstructionScript)

(fn SaveData
  (bind _returnvalue (SaveGame|DoesSaveGameExist (Variables|Default|GetSlot%20Name)))
  (if _returnvalue
    (bind _returnvalue_2 (SaveGame|LoadGamefromSlot (Variables|Default|GetSlot%20Name)))
    (bind _output_get (Variables|Default|SetSave _returnvalue_2))
    (bind _asdata_object (Utilities|Casting|CastToDataObject _output_get))
    (Default|LoadTime _asdata_object (Variables|Default|GetTimeMin) (Variables|Default|GetTimeSec))
    (else
      (bind _returnvalue_3 (SaveGame|CreateSaveGameObject "/Game/Blueprints/Character/DataObject.DataObject_C"))
      (bind _output_get_2 (Variables|Default|SetSave _returnvalue_3))
      (bind _asdata_object_2 (Utilities|Casting|CastToDataObject _output_get_2))
      (Default|LoadTime _asdata_object_2 (Variables|Default|GetTimeMin) (Variables|Default|GetTimeSec))))
  (SaveGame|SaveGametoSlot (Variables|Default|GetSave) (Variables|Default|GetSlot%20Name)))

(fn LoadData
  (bind _returnvalue (SaveGame|DoesSaveGameExist (Variables|Default|GetSlot%20Name)))
  (if _returnvalue
    (bind _returnvalue_2 (SaveGame|LoadGamefromSlot (Variables|Default|GetSlot%20Name)))
    (bind _output_get (Variables|Default|SetSave _returnvalue_2))
    (bind _asdata_object (Utilities|Casting|CastToDataObject _output_get))
    (Variables|Default|SetTimeMin (Variables|/Game/Blueprints/Character/DataObject.DataObject_C|GetTime%20MIn _asdata_object))
    (Variables|Default|SetTimeSec (Variables|/Game/Blueprints/Character/DataObject.DataObject_C|GetTime%20Sec _asdata_object))))